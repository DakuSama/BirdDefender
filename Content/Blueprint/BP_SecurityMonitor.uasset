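; BP_SecurityMonitor is an obsolete security monitor meant to display linked security camera feeds on its mesh.
; BeginPlay, the swap event and the construction script are empty, and all remaining logic is disconnected.
; That dead logic streams a camera's scene capture through a viewport-scaled render target into a dynamic material, cycling and rotating cameras.
; Other leftover fragments experiment with view-target switching and player look input.
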(event `self.ReceiveBeginPlay`
  ;[1 0.2532 0.9982] obselete
)

(event `EnhancedInput|/Game/Blueprint/Input/IA_Look`
  (params (ActionValue :type "Vector2D Structure") (ElapsedSeconds :type "Float (double-precision)") (TriggeredSeconds :type "Float (double-precision)") (InputAction :type "InputAction Object Reference" :default "/Game/Blueprint/Input/IA_Look.IA_Look"))
  ;[1 0.2532 0.9982] obselete
)

(event `EnhancedInput|/Game/Blueprint/Input/IA_Move`
  (params (ActionValue :type "Vector2D Structure") (ElapsedSeconds :type "Float (double-precision)") (TriggeredSeconds :type "Float (double-precision)") (InputAction :type "InputAction Object Reference" :default "/Game/Blueprint/Input/IA_Move.IA_Move"))
  ;[1 0.2532 0.9982] obselete
)

(event `EnhancedInput|/Game/Blueprint/Input/IA_Interact`
  (params (ActionValue :type Boolean) (ElapsedSeconds :type "Float (double-precision)") (TriggeredSeconds :type "Float (double-precision)") (InputAction :type "InputAction Object Reference" :default "/Game/Blueprint/Input/IA_Interact.IA_Interact"))
  ;[1 0.2532 0.9982] obselete
)

(event `SwapCameraObselet`
  ;[1 0.2532 0.9982] obselete
)

(fn `UserConstructionScript`)