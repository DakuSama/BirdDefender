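; BC_Clicked is a Blueprint component that lets the player damage its owning actor by clicking on it.
; On BeginPlay it binds to the owner's OnClicked event, and each click plays an attack sound and lowers the owner's Health by one.
; At zero Health it calls the owner's Death with SpawnerOrigine and prints the clicked actor's class name.
; An unconnected node that would decrement the spawner's CurrentNPC never runs.
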(event `self.ReceiveBeginPlay`
  (add `Actor.OnClicked` (`self.GetOwner`) (delegate `OnMouseClicked`)))

(event `OnMouseClicked`
  (params (TouchedActor :type "Actor Object Reference") (ButtonPressed :type "Key Structure" :default "None"))
  (bind _owner (`self.Owner`))
  (`GameplayStatics.PlaySound2D` "/Game/SFX/Player/SFX_Ch_LeftClickAttaque.SFX_Ch_LeftClickAttaque" 1.0 1.0 0.0 null null)
  (set `/Game/Blueprint/BP_AI/BP_IA_Base.Health` (- (`/Game/Blueprint/BP_AI/BP_IA_Base.Health` _owner) 1.0) _owner)
  (if (<= (`/Game/Blueprint/BP_AI/BP_IA_Base.Health` _owner) 0.0)
    (`/Game/Blueprint/BP_AI/BP_IA_Base.Death` _owner (`self.SpawnerOrigine`))
    (`KismetSystemLibrary.PrintString` (`KismetSystemLibrary.GetClassDisplayName` (`GameplayStatics.GetObjectClass` TouchedActor)) true true (struct :`R` 0.206295 :`G` 1.0 :`A` 1.0))))