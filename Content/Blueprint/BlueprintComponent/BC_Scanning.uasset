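; BC_Scanning is an actor component that handles cursor-hover scanning of AI and enemy prop actors.
; It binds to its owner's cursor-over events, starting the load scan only while the BPC_CameraManager is in scanning mode and ending it when the cursor leaves.
; A separate ResultaScan event resolves the scan by exact class, calling Scanning on BP_NPC or spawning an enemy from BP_PropsEnnemie.
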(event `self.ReceiveBeginPlay`
  (bind _returnvalue (`self.GetOwner`))
  (bind _outactors (`GameplayStatics.GetAllActorsOfClass` "/Game/Blueprint/BPC_CameraManager.BPC_CameraManager_C"))
  (set `self.CameraManager_REF` (`|GetArrayItem` _outactors))
  (add `Actor.OnBeginCursorOver` _returnvalue (delegate `BeginCursorOver`))
  (add `Actor.OnEndCursorOver` _returnvalue (delegate `EndCursorOver`)))

(event `EndCursorOver`
  (params (TouchedActor :type "Actor Object Reference"))
  (bind _asbp_ia_base (cast `/Game/Blueprint/BP_AI/BP_IA_Base` TouchedActor)
    (:`then`
      (`/Game/Blueprint/BP_AI/BP_IA_Base.EndLoadScan` _asbp_ia_base))
    (:`CastFailed`
      (bind _asbp_props_ennemie (cast `/Game/Blueprint/BP_AI/BP_PropsEnnemie` TouchedActor))
      (`/Game/Blueprint/BP_AI/BP_PropsEnnemie.EndLoadScan` _asbp_props_ennemie))))

(event `ResultaScan`
  (if (== (`GameplayStatics.GetObjectClass` (stale `BeginCursorOver` TouchedActor)) "/Game/Blueprint/BP_AI/BP_NPC.BP_NPC_C")
    (bind _asbp_npc (cast `/Game/Blueprint/BP_AI/BP_NPC` (stale `BeginCursorOver` TouchedActor)))
    (`/Game/Blueprint/BP_AI/BP_NPC.scanning` _asbp_npc)
    (elif (== (`GameplayStatics.GetObjectClass` (stale `BeginCursorOver` TouchedActor)) "/Game/Blueprint/BP_AI/BP_PropsEnnemie.BP_PropsEnnemie_C")
      (bind _asbp_props_ennemie (cast `/Game/Blueprint/BP_AI/BP_PropsEnnemie` (stale `BeginCursorOver` TouchedActor)))
      (`/Game/Blueprint/BP_AI/BP_PropsEnnemie.SpawnEnnemie` _asbp_props_ennemie))))

(event `BeginCursorOver`
  (params (TouchedActor :type "Actor Object Reference"))
  (if (`/Game/Blueprint/BPC_CameraManager.IsScanning?` (`self.CameraManager_REF`))
    (bind _asbp_ia_base (cast `/Game/Blueprint/BP_AI/BP_IA_Base` TouchedActor)
      (:`then`
        (`/Game/Blueprint/BP_AI/BP_IA_Base.BeginLoadScan` _asbp_ia_base))
      (:`CastFailed`
        (bind _asbp_props_ennemie (cast `/Game/Blueprint/BP_AI/BP_PropsEnnemie` TouchedActor))
        (`/Game/Blueprint/BP_AI/BP_PropsEnnemie.startLoadScan` _asbp_props_ennemie)))))