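; Enemy Blueprint that attacks generators, dealing damage to the nearest BP_Generator.
; On BeginPlay it applies its walk speed, enables custom depth on its static mesh and starts a looping timer that occasionally plays a random-chance voice line.
; Attack scans all generators for the closest by distance, plays an attack sound and applies its Damage to that one.
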(event `voice`
  (if (== (`KismetMathLibrary.RandomInteger` 10) 0)
    (`GameplayStatics.PlaySound2D` "/Game/SFX/ennemies/SW_Voice/Vo_en_FlappyVoice2.Vo_en_FlappyVoice2" 1.0 1.0 0.0 null null)))

(event `self.ReceiveBeginPlay`
  (`parent.ReceiveBeginPlay`)
  (set `CharacterMovementComponent.MaxWalkSpeed` (`self.Speed`) (`self.CharacterMovement`))
  (`PrimitiveComponent.SetRenderCustomDepth` (`self.StaticMesh`) true)
  (`KismetSystemLibrary.K2_SetTimerDelegate` (delegate `voice`) 5.0 true))

(event `/Game/Blueprint/BlueprintInterface/BPI_Attack.Attack`
  (bind _returnvalue (`PawnMovementComponent.GetPawnOwner` (`self.CharacterMovement`)))
  (bind _outactors (`GameplayStatics.GetAllActorsOfClass` "/Game/Blueprint/BP_LD/BP_Generator.BP_Generator_C"))
  (bind _output_get (set `self.GeneratorArray_0` _outactors))
  (set `self.MinDistance_0` (`self.GetDistanceTo` _returnvalue (`|GetArrayItem` _output_get)))
  (for (_array_element _array_index) _outactors
    (bind _output_get_2 (set `self.CurrentDistance_0` (`self.GetDistanceTo` _returnvalue _array_element)))
    (if (<= _output_get_2 (`self.MinDistance_0`))
      (set `self.MinDistance_0` (`self.CurrentDistance_0`))
      (set `self.MinIndex_0` _array_index)))
  (`GameplayStatics.PlaySound2D` "/Game/SFX/ennemies/SW_EnemiesAttack/SFX_EnemiesAttack_v3.SFX_EnemiesAttack_v3" 1.0 1.0 0.0 null null)
  (`GameplayStatics.ApplyDamage` (`|GetArrayItem` (`self.GeneratorArray_0`) (`self.MinIndex_0`)) (`self.Damage`) null self))

(fn `UserConstructionScript`
  (`parent.UserConstructionScript`))