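; Base AI character for NPCs and enemies, handling spawn setup, infection state, scanning feedback and death.
; BeginPlay passes its class to the Blackboard, randomly flags infection, enables custom depth and caches the nearest spawner and generator.
; A looping timer destroys it when its spawner's camera zone is inactive.
; Death decrements the spawner's count and plays effects, with NPC deaths also damaging the generator, while scanning drives timeline-based sound and Niagara effects.
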(event `self.ReceiveBeginPlay`
  (bind _returnvalue (`PawnMovementComponent.GetPawnOwner` (`self.CharacterMovement`)))
  (bind _returnvalue_2 (`PawnMovementComponent.GetPawnOwner` (`self.CharacterMovement`)))
  (bind _output (`|GetArrayItem` (`self.SpawnerArray`) (`self.MinIndex`)))
  (`BlackboardComponent.SetValueAsClass` (`AIBlueprintHelperLibrary.GetBlackboard` null) "ClassKey" (`GameplayStatics.GetObjectClass` self))
  (if (< (`KismetMathLibrary.RandomInteger` 10) 9)
    (set `self.IsInfected?` true))
  (`PrimitiveComponent.SetRenderCustomDepth` (`self.Mesh`) true)
  (bind _outactors (`GameplayStatics.GetAllActorsOfClass` "/Game/Blueprint/GM_CameraGame.GM_CameraGame_C"))
  (set `self.CameraGame_REF` (`|GetArrayItem` _outactors))
  (bind _outactors_2 (`GameplayStatics.GetAllActorsOfClass` "/Game/Blueprint/BPC_CameraManager.BPC_CameraManager_C"))
  (set `self.CameraManager_REF` (`|GetArrayItem` _outactors_2))
  (set `/Game/Blueprint/BlueprintComponent/BC_Clicked.Owner` self (`self.BC_Clicked`))
  (bind _outactors_3 (`GameplayStatics.GetAllActorsOfClass` "/Game/Blueprint/BP_AI/BP_Spawner.BP_Spawner_C"))
  (bind _output_get (set `self.SpawnerArray` _outactors_3))
  (set `self.MinDistance` (`self.GetDistanceTo` _returnvalue (`|GetArrayItem` _output_get)))
  (for (_array_element _array_index) _outactors_3
    (bind _output_get_2 (set `self.CurrentDistance` (`self.GetDistanceTo` _returnvalue _array_element)))
    (if (<= _output_get_2 (`self.MinDistance`))
      (set `self.MinDistance` (`self.CurrentDistance`))
      (set `self.MinIndex` _array_index)))
  (bind _output_get_3 (set `self.SpawnerOrigine` _output))
  (set `/Game/Blueprint/BlueprintComponent/BC_Clicked.SpawnerOrigine` _output_get_3 (`self.BC_Clicked`))
  (set `self.Index` (`/Game/Blueprint/BP_AI/BP_Spawner.CurrentIndex` _output))
  (`KismetSystemLibrary.K2_SetTimerDelegate` (delegate `CustomEvent`) 1.0 true)
  (bind _outactors_4 (`GameplayStatics.GetAllActorsOfClass` "/Game/Blueprint/BP_LD/BP_Generator.BP_Generator_C"))
  (bind _output_get_4 (set `self.GeneratorArray` _outactors_4))
  (set `self.MinDistance` (`self.GetDistanceTo` _returnvalue_2 (`|GetArrayItem` _output_get_4)))
  (for (_array_element_2 _array_index_2) _outactors_4
    (bind _output_get_5 (set `self.CurrentDistance` (`self.GetDistanceTo` _returnvalue_2 _array_element_2)))
    (if (<= _output_get_5 (`self.MinDistance`))
      (set `self.MinDistance` (`self.CurrentDistance`))
      (set `self.MinIndex` _array_index_2)))
  (set `self.Generator` (`|GetArrayItem` (`self.GeneratorArray`) (`self.MinIndex`))))

(event `CustomEvent`
  (if (not (`|GetArrayItem` (`/Game/Blueprint/GM_CameraGame.StateZone` (`self.CameraGame_REF`)) (`self.Index`)))
    (`self.K2_DestroyActor`)))

(event `Death`
  (params (`Spawner Origine` :type "/Game/Blueprint/BP_AI/BP_Spawner Object Reference"))
  (set `/Game/Blueprint/BP_AI/BP_Spawner.CurrentNPC` (- (`/Game/Blueprint/BP_AI/BP_Spawner.CurrentNPC` `Spawner Origine`) 1) `Spawner Origine`)
  (`MovementComponent.StopMovementImmediately` (`self.CharacterMovement`))
  (`GameplayStatics.PlaySound2D` "/Game/SFX/NPC/SFX_npc_Destroye.SFX_npc_Destroye" 0.4 1.0 0.0 null null)
  (if (== (`GameplayStatics.GetObjectClass` self) "/Game/Blueprint/BP_AI/BP_NPC.BP_NPC_C")
    (`GameplayStatics.ApplyDamage` (`self.Generator`) (`self.Base Damage`) null self)
    (`AddComponent|NODE_AddNiagaraComponent-5` :`bManualAttachment` true :`RelativeTransform` (`self.GetTransform`))
    (`SceneComponent.SetVisibility` (`self.StaticMesh`) false false :!label _label)
    (`SceneComponent.SetVisibility` (`self.Mesh`) false false)
    (`KismetSystemLibrary.Delay` 0.4)
    (`self.K2_DestroyActor`)
    (elif (== (`GameplayStatics.GetObjectClass` self) "/Game/Blueprint/BP_AI/BP_Ennemi.BP_Ennemi_C")
      (`AddComponent|NODE_AddNiagaraComponent-4` :`bManualAttachment` true :`RelativeTransform` (`self.GetTransform`))
      (goto _label))))

(event `BeginLoadScan`
  (bind _returnvalue (`GameplayStatics.SpawnSound2D` "/Game/SFX/Player/SFX_ScannerPlayer.SFX_ScannerPlayer" 1.0 1.0 0.0 null))
  (`Timeline|Timeline` :!label _label_2
    (:`Update`
      (`AddComponent|NODE_AddNiagaraComponent-6` :`bManualAttachment` true :`RelativeTransform` (`self.GetTransform`)))
    (:`Finished`
      (`AudioComponent.FadeOut` _returnvalue 0.0 0.0 "Linear"))))

(event `EndLoadScan`
  (goto _label_2 :!via `Stop`))

(fn `UserConstructionScript`)