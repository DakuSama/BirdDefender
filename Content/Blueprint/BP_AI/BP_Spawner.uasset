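; BP_Spawner is a timed spawner that creates AI pawns or enemy props while its game zone is active.
; A looping timer checks the zone state in GM_CameraGame at its index and counts spawns up to a maximum.
; Enemy and NPC classes spawn at the billboard with a shared base behavior tree.
; Any other class setting spawns BP_PropsEnnemie at a random reachable point around the spawner.
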(event `self.ReceiveBeginPlay`
  (`KismetSystemLibrary.K2_SetTimerDelegate` (delegate `Spawner`) (`self.Time`) true)
  (bind _outactors (`GameplayStatics.GetAllActorsOfClass` "/Game/Blueprint/GM_CameraGame.GM_CameraGame_C"))
  (set `self.GameModeREF` (`|GetArrayItem` _outactors)))

(event `Spawner`
  (bind _iaspawnable (`self.IASpawnable`))
  (if (`|GetArrayItem` (`/Game/Blueprint/GM_CameraGame.StateZone` (`self.GameModeREF`)) (`self.CurrentIndex`))
    (if (< (`self.CurrentNPC`) (`self.MaxNPC`))
      (set `self.CurrentNPC` (`KismetMathLibrary.Clamp` (+ (`self.CurrentNPC`) 1) 0 (`self.MaxNPC`)))
      (if (or (== _iaspawnable "/Game/Blueprint/BP_AI/BP_Ennemi.BP_Ennemi_C") (== _iaspawnable "/Game/Blueprint/BP_AI/BP_NPC.BP_NPC_C"))
        (`AIBlueprintHelperLibrary.SpawnAIFromClass` (`self.IASpawnable`) "/Game/Blueprint/BP_AI/IA/BT_IA_Base.BT_IA_Base" (`SceneComponent.K2_GetComponentLocation` (`self.Billboard`)) (struct) false null)
        (else
          (`|SpawnActorFromClass` "/Game/Blueprint/BP_AI/BP_PropsEnnemie.BP_PropsEnnemie_C" (`KismetMathLibrary.MakeTransform` (`NavigationSystemV1.K2_GetRandomReachablePointInRadius` (`self.K2_GetActorLocation`) 1000.0 null null)) "Undefined" "MultiplyWithRoot" null null))))))

(fn `UserConstructionScript`)