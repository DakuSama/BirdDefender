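; Scannable NPC that may be a disguised infected, turning into an enemy when scanned.
; On spawn it applies its walk speed, picks a random skin mesh and starts a looping timer that adds a Niagara effect above it every few seconds.
; Scanning an infected NPC plays a sound, spawns an AI-driven BP_Ennemi above it and calls Death with its origin spawner; otherwise only a scanned sound plays.
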(event `self.ReceiveBeginPlay`
  (`parent.ReceiveBeginPlay`)
  (set `CharacterMovementComponent.MaxWalkSpeed` (`self.Speed`) (`self.CharacterMovement`))
  (`SkeletalMeshComponent.SetSkeletalMeshAsset` (`self.Mesh`) (`|GetArrayItem` (`self.Skin`) (`KismetMathLibrary.RandomInteger` 5)))
  (`KismetSystemLibrary.K2_SetTimerDelegate` (delegate `CustomEvent_0`) 6.0 true))

(event `CustomEvent_0`
  (`AddComponent|NODE_AddNiagaraComponent-0` :`bManualAttachment` true :`RelativeTransform` (`KismetMathLibrary.MakeTransform` (+ (`self.K2_GetActorLocation`) (* (`KismetMathLibrary.GetUpVector` (struct)) 150.0)))))

(event `scanning`
  (if (`self.IsInfected?`)
    (`GameplayStatics.PlaySound2D` "/Game/SFX/ennemies/SFX_PropsToFlappy2.SFX_PropsToFlappy2" 1.0 1.0 0.0 null null)
    (`AIBlueprintHelperLibrary.SpawnAIFromClass` "/Game/Blueprint/BP_AI/BP_Ennemi.BP_Ennemi_C" "/Game/Blueprint/BP_AI/IA/BT_IA_Base.BT_IA_Base" (+ (`self.K2_GetActorLocation`) (* (`self.GetActorUpVector`) 150.0)) (struct) false null)
    (`self.Death` (`self.SpawnerOrigine`))
    (else
      (`GameplayStatics.PlaySound2D` "/Game/SFX/NPC/SFX_npc_Scanned.SFX_npc_Scanned" 1.0 1.0 0.0 null null))))

(fn `UserConstructionScript`
  (`parent.UserConstructionScript`))