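; BP_PropsEnnemie is a prop with a randomly picked mesh that turns into an AI enemy after a timer.
; When the timer fires, it plays a sound, spawns BP_Ennemi with the BT_IA_Base behavior tree above the mesh, then destroys itself.
; Separate scan events start a timeline with a scanner sound that is cut when it finishes, or stop the timeline early without cutting the sound.
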(event `self.ReceiveBeginPlay`
  (`StaticMeshComponent.SetStaticMesh` (`self.StaticMesh`) (`|GetArrayItem` (`self.Skin`) (`KismetMathLibrary.RandomInteger` (`KismetArrayLibrary.Array_Length` (`self.Skin`)))))
  (`KismetSystemLibrary.K2_SetTimerDelegate` (delegate `SpawnEnnemie`) (`self.Time`)))

(event `SpawnEnnemie`
  (bind _staticmesh (`self.StaticMesh`))
  (`GameplayStatics.PlaySound2D` "/Game/SFX/ennemies/SFX_PropsToFlappy.SFX_PropsToFlappy" 1.0 1.0 0.0 null null)
  (`AIBlueprintHelperLibrary.SpawnAIFromClass` "/Game/Blueprint/BP_AI/BP_Ennemi.BP_Ennemi_C" "/Game/Blueprint/BP_AI/IA/BT_IA_Base.BT_IA_Base" (+ (`SceneComponent.K2_GetComponentLocation` _staticmesh) (* (`SceneComponent.GetUpVector` _staticmesh) 150.0)) (struct) false null)
  (`self.K2_DestroyActor`))

(event `startLoadScan`
  (bind _returnvalue (`GameplayStatics.SpawnSound2D` "/Game/SFX/Player/SFX_ScannerPlayer.SFX_ScannerPlayer" 1.0 1.0 0.0 null))
  (`Timeline|Timeline` :!label _label
    (:`Finished`
      (`AudioComponent.FadeOut` _returnvalue 0.0 0.0 "Linear"))))

(event `EndLoadScan`
  (goto _label :!via `Stop`))

(fn `UserConstructionScript`)