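; Player controller that has the player possess and switch between the level's security cameras, clamping view angles on each possession.
; BeginPlay caches cameras and rotations and adds the HUD; Interact cycles feeds, buttons jump to one.
; Right-click zooms by FOV timeline except on camera zero, though mouse-look code is unwired.
; ClearCache wipes the current camera's NPCs and enemies, resets its spawners and toggles its state on timed cooldown; Escape toggles pause.
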(event `self.ReceiveBeginPlay`
  (`EnhancedInputSubsystemInterface.AddMappingContext` (pcsubsystem `EnhancedInputLocalPlayerSubsystem` self) "/Game/Blueprint/Input/IMC_Player.IMC_Player" 0 (struct))
  (bind _returnvalue (`|CreateWidget` "/Game/Blueprint/Widget/WBP_HUD.WBP_HUD_C" (`GameplayStatics.GetPlayerController` 0)))
  (bind _output_get (set `self.Widget_REF` _returnvalue))
  (`UserWidget.AddToViewport` _output_get 0)
  (bind _outactors (`GameplayStatics.GetAllActorsOfClass` "/Game/Blueprint/BP_SecurityCamera.BP_SecurityCamera_C"))
  (bind _output_get_2 (set `self.NewVar` _outactors))
  (for _array_element _output_get_2
    (bind _index (`/Game/Blueprint/BP_SecurityCamera.Index` _array_element))
    (`KismetArrayLibrary.Array_Set` (`self.RotationArray`) _index (`self.K2_GetActorRotation` _array_element))
    (`KismetArrayLibrary.Array_Set` (`self.CameraArray`) _index _array_element))
  (`self.Possess` (`|GetArrayItem` (`self.CameraArray`) (`self.CurrentCamera`)))
  (`GameplayStatics.PlaySound2D` "/Game/SFX/Player/SFX_AreaZoom.SFX_AreaZoom" 1.0 1.0 0.0 null null))

(event `EnhancedInput|/Game/Blueprint/Input/IA_RightClick`
  (params (ActionValue :type Boolean) (ElapsedSeconds :type "Float (double-precision)") (TriggeredSeconds :type "Float (double-precision)") (InputAction :type "InputAction Object Reference" :default "/Game/Blueprint/Input/IA_RightClick.IA_RightClick"))
  (bind _returnvalue (not (== (`self.CurrentCamera`) 0)))
  (:`Started`
    (if _returnvalue
      (set `self.IsScanning?` true)
      (`self.SetControlRotation` (`KismetMathLibrary.FindLookAtRotation` (`self.K2_GetActorLocation`) (`.WorldDirection` (`self.DeprojectMousePositionToWorld` self))))
      (bind (_direction _zoom) (`Timeline|Zoom` :!label _label)
        (:`Update`
          (`CameraComponent.SetFieldOfView` (`/Game/Blueprint/BP_SecurityCamera.Camera` (`|GetArrayItem` (`self.CameraArray`) (`self.CurrentCamera`))) (`KismetMathLibrary.Lerp` 90.0 40.0 _zoom))))))
  (:`Completed`
    (if _returnvalue
      (set `self.IsScanning?` false)
      (`self.SetControlRotation` (`|GetArrayItem` (`self.RotationArray`) (`self.CurrentCamera`)))
      (goto _label :!via `Reverse`))))

(event `EnhancedInput|/Game/Blueprint/Input/IA_Move`
  (params (ActionValue :type "Vector2D Structure") (ElapsedSeconds :type "Float (double-precision)") (TriggeredSeconds :type "Float (double-precision)") (InputAction :type "InputAction Object Reference" :default "/Game/Blueprint/Input/IA_Move.IA_Move")))

(event `EnhancedInput|/Game/Blueprint/Input/IA_Look`
  (params (ActionValue :type "Vector2D Structure") (ElapsedSeconds :type "Float (double-precision)") (TriggeredSeconds :type "Float (double-precision)") (InputAction :type "InputAction Object Reference" :default "/Game/Blueprint/Input/IA_Look.IA_Look")))

(event `EnhancedInput|/Game/Blueprint/Input/IA_LeftClick`
  (params (ActionValue :type Boolean) (ElapsedSeconds :type "Float (double-precision)") (TriggeredSeconds :type "Float (double-precision)") (InputAction :type "InputAction Object Reference" :default "/Game/Blueprint/Input/IA_LeftClick.IA_LeftClick"))
  ;[1 1 1] Input
)

(event `ClearCache`
  (bind _currentcamera (`self.CurrentCamera`))
  ;[0.04229 1 0] Code Clear Cache
  (if (`self.IsClear?`)
    (set `self.IsClear?` false)
    (bind _outactors (`GameplayStatics.GetAllActorsOfClass` "/Game/Blueprint/BP_AI/BP_NPC.BP_NPC_C"))
    (for _array_element _outactors
      (if (== (`/Game/Blueprint/BP_AI/BP_IA_Base.Index` _array_element) (`self.CurrentCamera`))
        (`self.K2_DestroyActor` _array_element)))
    (bind _outactors_2 (`GameplayStatics.GetAllActorsOfClass` "/Game/Blueprint/BP_AI/BP_Ennemi.BP_Ennemi_C"))
    (for _array_element_2 _outactors_2
      (if (== (`/Game/Blueprint/BP_AI/BP_IA_Base.Index` _array_element_2) (`self.CurrentCamera`))
        (`self.K2_DestroyActor` _array_element_2)))
    (bind _outactors_3 (`GameplayStatics.GetAllActorsOfClass` "/Game/Blueprint/BP_AI/BP_Spawner.BP_Spawner_C"))
    (for _array_element_3 _outactors_3
      (if (== (`/Game/Blueprint/BP_AI/BP_Spawner.CurrentIndex` _array_element_3) (`self.CurrentCamera`))
        (set `/Game/Blueprint/BP_AI/BP_Spawner.CurrentNPC` 0 _array_element_3)))
    (`KismetArrayLibrary.Array_Set` (`self.StateCamera`) _currentcamera)
    (`KismetArrayLibrary.Array_AddUnique` (`self.SaveCameraCache`) _currentcamera)
    (`KismetSystemLibrary.Delay` 10.0)
    (`KismetArrayLibrary.Array_Set` (`self.StateCamera`) (`|GetArrayItem` (`self.SaveCameraCache`)) true)
    (`KismetArrayLibrary.Array_Clear` (`self.SaveCameraCache`))
    (`KismetSystemLibrary.Delay` 53.0)
    (set `self.IsClear?` true)))

(event `EnhancedInput|/Game/Blueprint/Input/IA_Interact`
  (params (ActionValue :type Boolean) (ElapsedSeconds :type "Float (double-precision)") (TriggeredSeconds :type "Float (double-precision)") (InputAction :type "InputAction Object Reference" :default "/Game/Blueprint/Input/IA_Interact.IA_Interact"))
  (bind _currentcamera (`self.CurrentCamera`))
  (bind _currentcamera_2 (`self.CurrentCamera`))
  (:`Started`
    (`KismetArrayLibrary.Array_Set` (`self.RotationArray`) (`self.CurrentCamera`) (`self.GetControlRotation`))
    (`/Engine/EditorBlueprintResources/StandardMacros.IncrementInt` _currentcamera
      (:`  `
        (if (>= _currentcamera (`KismetArrayLibrary.Array_Length` (`self.CameraArray`)))
          (set `self.CurrentCamera` 0))
        (`self.Possess` (`|GetArrayItem` (`self.CameraArray`) _currentcamera_2))
        (`GameplayStatics.PlaySound2D` "/Game/SFX/Player/SFX_AreaZoom.SFX_AreaZoom" 1.0 1.0 0.0 null null)
        (`self.SetControlRotation` (`|GetArrayItem` (`self.RotationArray`) _currentcamera_2))))))

(event `button_0`
  ;[1 1 1] Input
  (set `self.CurrentCamera` 0)
  (`self.Possess` (`|GetArrayItem` (`self.CameraArray`)))
  (`GameplayStatics.PlaySound2D` "/Game/SFX/Player/SFX_AreaZoom.SFX_AreaZoom" 1.0 1.0 0.0 null null))

(event `button_1`
  ;[1 1 1] Input
  (set `self.CurrentCamera` 1)
  (`self.Possess` (`|GetArrayItem` (`self.CameraArray`) 1))
  (`GameplayStatics.PlaySound2D` "/Game/SFX/Player/SFX_AreaZoom.SFX_AreaZoom" 1.0 1.0 0.0 null null))

(event `self.ReceivePossess`
  (params (PossessedPawn :type "Pawn Object Reference"))
  (`self.ClampView` PossessedPawn))

(event `button_2`
  ;[1 1 1] Input
  (set `self.CurrentCamera` 2)
  (`self.Possess` (`|GetArrayItem` (`self.CameraArray`) 2))
  (`GameplayStatics.PlaySound2D` "/Game/SFX/Player/SFX_AreaZoom.SFX_AreaZoom" 1.0 1.0 0.0 null null))

(event `EnhancedInput|/Game/Blueprint/Input/IA_Echap`
  (params (ActionValue :type Boolean) (ElapsedSeconds :type "Float (double-precision)") (TriggeredSeconds :type "Float (double-precision)") (InputAction :type "InputAction Object Reference" :default "/Game/Blueprint/Input/IA_Echap.IA_Echap"))
  (:`Started`
    (if (not (`self.isPauseMenuOpened?`))
      (set `self.isPauseMenuOpened?` true)
      (bind _returnvalue (`|CreateWidget` "/Game/Blueprint/Widget/WBP_PauseMenu.WBP_PauseMenu_C" (`GameplayStatics.GetPlayerController` 0)))
      (bind _output_get (set `self.PauseMenuWidget` _returnvalue))
      (`UserWidget.AddToViewport` _output_get 0)
      (`GameplayStatics.PlaySound2D` "/Game/SFX/UI/SFX_ui_OpenPauseMenu.SFX_ui_OpenPauseMenu" 1.0 1.0 0.0 null null)
      (`GameplayStatics.SetGamePaused` true)
      (else
        (set `self.isPauseMenuOpened?` false)
        (`Widget.RemoveFromParent` (`self.PauseMenuWidget`))
        (`GameplayStatics.SetGamePaused` false)))))

(event `button_3`
  ;[1 1 1] Input
  (set `self.CurrentCamera` 3)
  (`self.Possess` (`|GetArrayItem` (`self.CameraArray`) 3))
  (`GameplayStatics.PlaySound2D` "/Game/SFX/Player/SFX_AreaZoom.SFX_AreaZoom" 1.0 1.0 0.0 null null))

(event `button_4`
  ;[1 1 1] Input
  (set `self.CurrentCamera` 4)
  (`self.Possess` (`|GetArrayItem` (`self.CameraArray`) 4))
  (`GameplayStatics.PlaySound2D` "/Game/SFX/Player/SFX_AreaZoom.SFX_AreaZoom" 1.0 1.0 0.0 null null))

(fn `ClampView`
  (params (self2 :type "Actor Object Reference"))
  (bind (_returnvalue_roll _returnvalue_pitch) (`KismetMathLibrary.BreakRotator` (`self.K2_GetActorRotation` self2)))
  (bind (_returnvalue_roll_2 _returnvalue_pitch_2) (`KismetMathLibrary.BreakRotator` (`self.K2_GetActorRotation` self2)))
  (bind (_returnvalue_roll_3 _returnvalue_pitch_3 _returnvalue_yaw) (`KismetMathLibrary.BreakRotator` (`self.K2_GetActorRotation` self2)))
  (bind _returnvalue (`GameplayStatics.GetPlayerCameraManager` 0))
  (bind (_returnvalue_roll_4 _returnvalue_pitch_4 _returnvalue_yaw_2) (`KismetMathLibrary.BreakRotator` (`self.K2_GetActorRotation` self2)))
  (set `PlayerCameraManager.ViewPitchMin` (- _returnvalue_pitch (`self.MinPitch`)) _returnvalue)
  (set `PlayerCameraManager.ViewPitchMax` (+ _returnvalue_pitch_2 (`self.MaxPitch`)) _returnvalue)
  (set `PlayerCameraManager.ViewYawMin` (- _returnvalue_yaw_2 (`self.MinYaw`)) _returnvalue)
  (set `PlayerCameraManager.ViewYawMax` (+ _returnvalue_yaw (`self.MaxYaw`)) _returnvalue))

(fn `UserConstructionScript`)