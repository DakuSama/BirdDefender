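; Game mode for a camera game in which the player survives a countdown while keeping generators intact.
; A Delay on Tick throttles the minute and second countdown, and a looping timer shows the win widget when it reaches zero.
; Another timer polls BP_Generator actors and triggers game over if fewer than four remain.
; An early one-shot and a recurring timer flag successive StateZone entries with a security sound, and both endings pause play and swap audio.
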(event `self.ReceiveTick`
  (params (DeltaSeconds :type "Float (single-precision)"))
  (`KismetSystemLibrary.Delay` 1.0)
  (if (== (`self.CurrentSeconds`) 0)
    (if (not (== (`self.CurrentMinutes`) 0))
      (set `self.CurrentSeconds` 59)
      (set `self.CurrentMinutes` (- (`self.CurrentMinutes`) 1)))
    (else
      (set `self.CurrentSeconds` (- (`self.CurrentSeconds`) 1)))))

(event `self.ReceiveBeginPlay`
  (`WidgetBlueprintLibrary.SetInputMode_GameAndUIEx` (`GameplayStatics.GetPlayerController` 0) null "DoNotLock" false)
  (set `self.CurrentMinutes` (`self.MaxMinutes`))
  (`KismetSystemLibrary.K2_SetTimerDelegate` (delegate `CheckNumberGenerator`) 0.5 true)
  (`KismetSystemLibrary.K2_SetTimerDelegate` (delegate `CustomEvent_0`) 10.0)
  (`KismetSystemLibrary.K2_SetTimerDelegate` (delegate `Increment Stack Lock`) 60.0 true)
  (`KismetSystemLibrary.K2_SetTimerDelegate` (delegate `CustomEvent`) 1.0 true)
  (bind _returnvalue (`GameplayStatics.SpawnSound2D` "/Game/SFX/SFX_music_gameover_Lp.SFX_music_gameover_Lp" 0.05 1.0 0.0 null))
  (set `self.sfx` _returnvalue))

(event `Increment Stack Lock`
  (set `self.StakLock` (+ (`self.StakLock`) 1))
  (`KismetArrayLibrary.Array_Set` (`self.StateZone`) (`self.StakLock`) true)
  (`GameplayStatics.PlaySound2D` "/Game/SFX/UI/SFX_UI_SecurityNoVoice.SFX_UI_SecurityNoVoice" 1.0 1.0 0.0 null null))

(event `CustomEvent_0`
  (`self.Increment Stack Lock`))

(event `CustomEvent`
  (if (and (== (`self.CurrentMinutes`) 0) (== (`self.CurrentSeconds`) 0))
    (`GameplayStatics.SetGamePaused` true)
    (bind _returnvalue (`|CreateWidget` "/Game/Blueprint/Widget/WBP_Win.WBP_Win_C"))
    (`UserWidget.AddToViewport` _returnvalue 0)
    (`AudioComponent.FadeOut` (`self.sfx`) 0.0 0.0 "Linear")
    (`GameplayStatics.SpawnSound2D` "/Game/SFX/UI/SFX_UI_VictoryVoiceActor.SFX_UI_VictoryVoiceActor" 100.0 1.0 0.0 null)))

(event `CheckNumberGenerator`
  (bind _outactors (`GameplayStatics.GetAllActorsOfClass` "/Game/Blueprint/BP_LD/BP_Generator.BP_Generator_C"))
  (if (< (`KismetArrayLibrary.Array_Length` _outactors) 4)
    (`GameplayStatics.SetGamePaused` true)
    (bind _returnvalue (`|CreateWidget` "/Game/Blueprint/Widget/WBP_GameOver.WBP_GameOver_C"))
    (`UserWidget.AddToViewport` _returnvalue 0)
    (`AudioComponent.FadeOut` (`self.sfx`) 0.0 0.0 "Linear")
    (`GameplayStatics.SpawnSound2D` "/Game/SFX/SFX_music_menu_Lp-001.SFX_music_menu_Lp-001" 0.5 1.0 0.0 null)))

(fn `UserConstructionScript`)