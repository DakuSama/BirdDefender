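; BP_AreaWall is a level design Blueprint that builds a straight wall of static meshes from its local origin to an EndPoint.
; The construction script divides that distance by a segment length and adds mesh components at that spacing, each rotated toward EndPoint.
; Each segment gets a random mesh from the StaticMesh array, with no fixed seed, so the mix can change whenever construction reruns.
; The event graph has no active logic.
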(fn `UserConstructionScript`
  (for _index (range (+ (- (`KismetMathLibrary.FTrunc` (/ (`KismetMathLibrary.Vector_Distance` (`KismetMathLibrary.MakeVector` 0.0) (`self.EndPoint`)) (`self.Lenght`))) 0) 1))
    (bind _returnvalue (`AddComponent|NODE_AddStaticMeshComponent-0` :`RelativeTransform` (`KismetMathLibrary.MakeTransform` (* (`KismetMathLibrary.GetDirectionUnitVector` (`KismetMathLibrary.MakeVector` 0.0) (`self.EndPoint`)) (`self.Lenght`) _index) (`KismetMathLibrary.FindLookAtRotation` (`KismetMathLibrary.MakeVector` 0.0) (`self.EndPoint`)))))
    (`StaticMeshComponent.SetStaticMesh` _returnvalue (`KismetArrayLibrary.Array_Random` (`self.StaticMesh`)))))