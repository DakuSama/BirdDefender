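; BP_Generator is a destructible generator actor with health, a skin mesh picked by index and a health bar widget.
; Damage lowers health and updates the bar, or plays an explosion sound and destroys the actor at zero.
; A slow looping timer regenerates health without refreshing the bar, while a faster one turns the widget toward the player controller's location.
; The mesh renders to custom depth.
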(event `self.ReceiveBeginPlay`
  (set `self.CurrentHealth` (`self.MaxHealth`))
  (bind _aswbp_health_bar_generator (cast `/Game/Blueprint/Widget/WBP_HealthBarGenerator` (`WidgetComponent.GetWidget` (`self.Widget`))))
  (set `self.HealthBarWidgetREF` _aswbp_health_bar_generator)
  (`KismetSystemLibrary.K2_SetTimerDelegate` (delegate `UpdateWidgetrotation`) 0.2 true)
  (`StaticMeshComponent.SetStaticMesh` (`self.StaticMesh`) (`|GetArrayItem` (`self.Skin`) (`self.Index`)))
  (`PrimitiveComponent.SetMaterial` (`self.StaticMesh`) 0 "/Game/Mesh/LD/Mesh/Enviro_LAB/Texture/Lab_TX_Mat.Lab_TX_Mat")
  (`PrimitiveComponent.SetRenderCustomDepth` (`self.StaticMesh`) true)
  (`KismetSystemLibrary.K2_SetTimerDelegate` (delegate `CustomEvent`) 10.0 true))

(event `UpdateWidgetrotation`
  (`SceneComponent.K2_SetWorldRotation` (`self.Widget`) (`KismetMathLibrary.FindLookAtRotation` (`self.K2_GetActorLocation`) (`self.K2_GetActorLocation` (`GameplayStatics.GetPlayerController` 0))) false false))

(event `CustomEvent`
  (set `self.CurrentHealth` (`KismetMathLibrary.FClamp` (+ (`self.CurrentHealth`) 1.0) 0.0 (`self.MaxHealth`))))

(event `self.ReceiveAnyDamage`
  (params (Damage :type "Float (single-precision)") (DamageType :type "DamageType Object Reference") (InstigatedBy :type "Controller Object Reference") (DamageCauser :type "Actor Object Reference"))
  (bind _output_get (set `self.CurrentHealth` (`KismetMathLibrary.FClamp` (- (`self.CurrentHealth`) Damage) 0.0 (`self.MaxHealth`))))
  (if (<= _output_get 0.0)
    (`GameplayStatics.PlaySound2D` "/Game/SFX/UI/SFX_ExplosionPointVitale.SFX_ExplosionPointVitale" 0.5 1.0 0.0 null null)
    (`self.K2_DestroyActor`)
    (else
      (`/Game/Blueprint/Widget/WBP_HealthBarGenerator.Update Health` (`self.HealthBarWidgetREF`) (/ (`self.CurrentHealth`) (`self.MaxHealth`))))))

(fn `UserConstructionScript`)